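; Player character Blueprint for an action game, handling movement, stamina-gated combat and death.
; Inputs set timed state flags for light attack, immune directional dash flowing into run, and a Sweep Stun ability granting a shield.
; Damage hits shield, then health, and builds points for a temporary Legend State with alternate attacks, faster movement and regeneration.
; Tick uses Delay to throttle stamina drain and recovery; death pauses into a menu.
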(event `Key|H`
  (params (Key :type "Key Structure"))
  ;[1 1 1] CHEAT
)

(event `Key|J`
  (params (Key :type "Key Structure"))
  ;[1 1 1] CHEAT
)

(event `Key|K`
  (params (Key :type "Key Structure"))
  ;[1 1 1] CHEAT
)

(event `Key|L`
  (params (Key :type "Key Structure"))
  ;[1 1 1] CHEAT
)

(event `InputAction|Attack`
  (params (Key :type "Key Structure"))
  ;[1 1 1] ATTACK
  (:`Pressed`
    (if (`self.LegendStateActivation`)
      _
      (elif (and (>= (`self.CurrentStamina`) 10.0) (`self.LightAttackReady`) (`self.AbilityEReady`) (not (`self.LightAttackDelay`)))
        (if (`self.LegendState`)
          (set `self.LightAttack_LegendState` true)
          (set `self.LightAttackReady` false)
          (set `self.IsRunning` false)
          (set `self.LightAttackDelay` true)
          (set `self.CurrentStamina` (- (`self.CurrentStamina`) 10.0))
          (`CharacterMovementComponent.DisableMovement` (`self.CharacterMovement`))
          (`KismetSystemLibrary.Delay` 0.65)
          (`CharacterMovementComponent.SetMovementMode` (`self.CharacterMovement`) "MOVE_Walking" 0)
          (set `self.LightAttack_LegendState` false)
          (set `self.LightAttackReady` true)
          (set `self.LightAttackDelay` false)
          (else
            (set `self.LightAttack` true)
            (set `self.LightAttackReady` false)
            (set `self.IsRunning` false)
            (set `self.LightAttackDelay` true)
            (set `self.CurrentStamina` (- (`self.CurrentStamina`) 10.0))
            (`CharacterMovementComponent.DisableMovement` (`self.CharacterMovement`))
            (`KismetSystemLibrary.Delay` 0.65)
            (`CharacterMovementComponent.SetMovementMode` (`self.CharacterMovement`) "MOVE_Walking" 0)
            (set `self.LightAttack` false)
            (set `self.LightAttackReady` true)
            (set `self.LightAttackDelay` false)))))))

(event `Key|LeftAlt`
  (params (Key :type "Key Structure")))

(event `InputAxis|Move_ForwardBackward`
  (params (AxisValue :type "Float (single-precision)"))
  ;[0.8021 0.8013 0.7534] BASIC MOVEMENT
  (bind _output_get (set `self.ForwardIndex` AxisValue))
  (`self.AddMovementInput` (`self.GetActorForwardVector`) _output_get))

(event `InputAxis|Rotate_UpDown`
  (params (AxisValue :type "Float (single-precision)"))
  ;[0.8021 0.8013 0.7534] BASIC MOVEMENT
  (`self.AddControllerPitchInput` AxisValue))

(event `InputAxis|Rotate_RightLeft`
  (params (AxisValue :type "Float (single-precision)"))
  ;[0.8021 0.8013 0.7534] BASIC MOVEMENT
  (`self.AddControllerYawInput` AxisValue))

(event `InputAction|Legend State`
  (params (Key :type "Key Structure"))
  ;[0.8333 0.3559 0.3869] LEGEND STATE
  (:`Pressed`
    (if (or (`self.AbilityE`) (`self.AbilityE_LegendState`) (not (`self.LightAttackReady`)))
      _
      (elif (>= (`self.LegendStatePoints`) 100.0)
        (`|ExecutionSequence`
          (:`then_0`
            (set `self.LegendState` true)
            (set `self.IsRunning` false)
            (`KismetSystemLibrary.PrintString` "LEGEND STATE")
            (`|ExecutionSequence`
              (:`then_0`
                (set `self.LegendStatePoints` 0.0)
                (`KismetSystemLibrary.Delay` 10.0)
                (set `self.LegendState` false)
                (`KismetSystemLibrary.PrintString` "LEGEND STATE IS OVER"))
              (:`then_1`
                (set `self.CurrentStamina` (+ (`self.CurrentStamina`) (* (`self.RecoverStamina`) 2.0))))
              (:`then_2`
                (`CharacterMovementComponent.DisableMovement` (`self.CharacterMovement`))
                (`KismetSystemLibrary.Delay` 2.06)
                (`CharacterMovementComponent.SetMovementMode` (`self.CharacterMovement`) "MOVE_Walking" 0))))
          (:`then_1`
            (set `self.LegendStateActivation` true)
            (`KismetSystemLibrary.Delay` 2.06)
            (set `self.LegendStateActivation` false)))))))

(event `InputAxis|Move_RightLeft`
  (params (AxisValue :type "Float (single-precision)"))
  ;[0.8021 0.8013 0.7534] BASIC MOVEMENT
  (if (not (`self.DisableAD`))
    (bind _output_get (set `self.RightIndex` AxisValue))
    (`self.AddMovementInput` (`self.GetActorRightVector`) _output_get)))

(event `InputAction|Dash`
  (params (Key :type "Key Structure"))
  (bind _charactermovement (`self.CharacterMovement`))
  ;[0.4463 0.9602 1] DASH
  (:`Pressed`
    (if (or (`self.LegendStateActivation`) (`self.AbilityE`) (`self.AbilityE_LegendState`) (`self.IsRunning`) (`self.DashCooldown`) (`self.LightAttack`))
      _
      (elif (>= (`self.CurrentStamina`) 5.0)
        (`/Engine/EditorBlueprintResources/StandardMacros.DoOnce` false :!label _label
          (:`Completed`
            (set `self.CurrentStamina` (- (`self.CurrentStamina`) 5.0))
            (set `self.isImmune` true)
            (`KismetSystemLibrary.PrintString` "IS IMMUNE")
            (`|ExecutionSequence`
              (:`then_0`
                (if (>= (`self.ForwardIndex`) 1.0)
                  (set `self.DashF` true)
                  (set `self.DashCooldown` true)
                  (`self.LaunchCharacter` (* (`SceneComponent.GetForwardVector` (`self.CapsuleComponent`)) 7000.0))
                  (`KismetSystemLibrary.Delay` 0.9)
                  (set `self.DashF` false)
                  (set `self.DashCooldown` false)
                  (set `self.isImmune` false)
                  (`KismetSystemLibrary.PrintString` "IS NOT IMMUNE")
                  (`KismetSystemLibrary.Delay` 0.2)
                  (goto _label :!via `Reset`)))
              (:`then_1`
                (if (<= (`self.ForwardIndex`) -1.0)
                  (set `self.DashB` true)
                  (set `self.DashCooldown` true)
                  (`self.LaunchCharacter` (* (`SceneComponent.GetForwardVector` (`self.CapsuleComponent`)) -7000.0))
                  (`KismetSystemLibrary.Delay` 0.9)
                  (set `self.DashB` false)
                  (set `self.DashCooldown` false)
                  (set `self.isImmune` false)
                  (`KismetSystemLibrary.PrintString` "IS NOT IMMUNE")
                  (`KismetSystemLibrary.Delay` 0.2)
                  (goto _label :!via `Reset`)))
              (:`then_2`
                (if (>= (`self.RightIndex`) 1.0)
                  (set `self.DashR` true)
                  (set `self.DashCooldown` true)
                  (`self.LaunchCharacter` (* (`SceneComponent.GetRightVector` (`self.CapsuleComponent`)) 7000.0))
                  (`KismetSystemLibrary.Delay` 0.9)
                  (set `self.DashR` false)
                  (set `self.DashCooldown` false)
                  (set `self.isImmune` false)
                  (`KismetSystemLibrary.PrintString` "IS NOT IMMUNE")
                  (`KismetSystemLibrary.Delay` 0.2)
                  (goto _label :!via `Reset`)))
              (:`then_3`
                (if (<= (`self.RightIndex`) -1.0)
                  (set `self.DashL` true)
                  (set `self.DashCooldown` true)
                  (`self.LaunchCharacter` (* (`SceneComponent.GetRightVector` (`self.CapsuleComponent`)) -7000.0))
                  (`KismetSystemLibrary.Delay` 0.9)
                  (set `self.DashL` false)
                  (set `self.DashCooldown` false)
                  (set `self.isImmune` false)
                  (`KismetSystemLibrary.PrintString` "IS NOT IMMUNE")
                  (`KismetSystemLibrary.Delay` 0.2)
                  (goto _label :!via `Reset`)))
              (:`then_4`
                ;[1 1 1] RUN
                (`KismetSystemLibrary.Delay` 0.55)
                (if (and (> (`self.CurrentStamina`) 0.0) (> (`self.ForwardIndex`) 0.0))
                  (set `self.IsRunning` true)
                  (set `self.DisableAD` true)
                  (if (`self.LegendState`)
                    ;;[1 1 1] LEGEND STATE RUN
                    (set `CharacterMovementComponent.MaxWalkSpeed` 2250.0 _charactermovement)
                    (else
                      (set `CharacterMovementComponent.MaxWalkSpeed` 1500.0 _charactermovement))))))))
        (elif (and (< (`self.CurrentStamina`) 5.0) (> (`self.CurrentStamina`) 0.0))
          (`/Engine/EditorBlueprintResources/StandardMacros.DoOnce` false :!label _label_2
            (:`Completed`
              (set `self.CurrentStamina` (- (`self.CurrentStamina`) (`self.CurrentStamina`)))
              (`|ExecutionSequence`
                (:`then_0`
                  (if (>= (`self.ForwardIndex`) 1.0)
                    (set `self.DashF` true)
                    (`self.LaunchCharacter` (* (`SceneComponent.GetForwardVector` (`self.CapsuleComponent`)) 3750.0))
                    (`KismetSystemLibrary.Delay` 0.9)
                    (set `self.DashF` false)
                    (set `self.isImmune` false)
                    (`KismetSystemLibrary.PrintString` "IS NOT IMMUNE")
                    (`KismetSystemLibrary.Delay` 0.2)
                    (goto _label_2 :!via `Reset`)))
                (:`then_1`
                  (if (<= (`self.ForwardIndex`) -1.0)
                    (set `self.DashB` true)
                    (`self.LaunchCharacter` (* (`SceneComponent.GetForwardVector` (`self.CapsuleComponent`)) -3750.0))
                    (`KismetSystemLibrary.Delay` 0.9)
                    (set `self.DashB` false)
                    (set `self.isImmune` false)
                    (`KismetSystemLibrary.PrintString` "IS NOT IMMUNE")
                    (`KismetSystemLibrary.Delay` 0.2)
                    (goto _label_2 :!via `Reset`)))
                (:`then_2`
                  (if (>= (`self.RightIndex`) 1.0)
                    (set `self.DashR` true)
                    (`self.LaunchCharacter` (* (`SceneComponent.GetRightVector` (`self.CapsuleComponent`)) 3750.0))
                    (`KismetSystemLibrary.Delay` 0.9)
                    (set `self.DashR` false)
                    (set `self.isImmune` false)
                    (`KismetSystemLibrary.PrintString` "IS NOT IMMUNE")
                    (`KismetSystemLibrary.Delay` 0.2)
                    (goto _label_2 :!via `Reset`)))
                (:`then_3`
                  (if (<= (`self.RightIndex`) -1.0)
                    (set `self.DashL` true)
                    (`self.LaunchCharacter` (* (`SceneComponent.GetRightVector` (`self.CapsuleComponent`)) -3750.0))
                    (`KismetSystemLibrary.Delay` 0.9)
                    (set `self.DashL` false)
                    (set `self.isImmune` false)
                    (`KismetSystemLibrary.PrintString` "IS NOT IMMUNE")
                    (`KismetSystemLibrary.Delay` 0.2)
                    (goto _label_2 :!via `Reset`)))))))))))

(event `Key|E`
  (params (Key :type "Key Structure"))
  ;[1 1 1] ABILITY Sweep Stun
  (:`Pressed`
    (if (and (not (`self.AbilityE_Cooldown`)) (not (`self.LegendStateActivation`)) (`self.AbilityEReady`) (`self.LightAttackReady`) (<= (`self.AbilityECooldown`) 0.0))
      (if (>= (`self.CurrentStamina`) 15.0)
        (set `self.CurrentStamina` (- (`self.CurrentStamina`) 15.0))
        (`|ExecutionSequence`
          (:`then_0`
            (if (`self.LegendState`)
              (set `self.AbilityEReady` false)
              (set `self.AbilityE_LegendState` true)
              (set `self.IsRunning` false)
              (`CharacterMovementComponent.DisableMovement` (`self.CharacterMovement`))
              (`KismetSystemLibrary.Delay` 0.8)
              (set `self.AbilityE_LegendState` false)
              (`CharacterMovementComponent.SetMovementMode` (`self.CharacterMovement`) "MOVE_Walking" 0)
              (set `self.AbilityEReady` true)
              (`KismetSystemLibrary.PrintString` "Sweep Stun LS")
              (else
                (set `self.AbilityEReady` false)
                (set `self.AbilityE` true)
                (set `self.IsRunning` false)
                (`CharacterMovementComponent.DisableMovement` (`self.CharacterMovement`))
                (`KismetSystemLibrary.Delay` 0.8)
                (set `self.AbilityE` false)
                (`CharacterMovementComponent.SetMovementMode` (`self.CharacterMovement`) "MOVE_Walking" 0)
                (set `self.AbilityEReady` true)
                (`KismetSystemLibrary.PrintString` "Sweep Stun"))))
          (:`then_1`
            (set `self.AbilityE_Cooldown` true)
            (`KismetSystemLibrary.Delay` 8.0)
            (set `self.AbilityE_Cooldown` false))
          (:`then_2`
            (set `self.Shield` 30.0))
          (:`then_3`
            (set `self.AbilityECooldown` 1.0)
            (if (> (`self.AbilityECooldown`) 0.0) :!label _label_3
              (set `self.AbilityECooldown` (- (`self.AbilityECooldown`) 0.00625))
              (`KismetSystemLibrary.Delay` 0.05)
              (goto _label_3))))))))

(event `InputAction|Run`
  (params (Key :type "Key Structure"))
  ;[1 1 1] RUN
)

(event `Key|W`
  (params (Key :type "Key Structure"))
  (bind _charactermovement (`self.CharacterMovement`))
  ;[1 1 1] RUN
  (:`Released`
    (set `self.IsRunning` false :!label _label_4)
    (set `self.DisableAD` false)
    (if (`self.LegendState`)
      (set `CharacterMovementComponent.MaxWalkSpeed` 1350.0 _charactermovement)
      (else
        (set `CharacterMovementComponent.MaxWalkSpeed` 900.0 _charactermovement)))))

(event `Key|S`
  (params (Key :type "Key Structure"))
  ;[1 1 1] RUN
  (:`Pressed`
    (goto _label_4)))

(event `self.ReceiveTick`
  (params (DeltaSeconds :type "Float (single-precision)"))
  ;[1 0.9498 0.3181] RECOVER STAMINA & DECREASE WHEN RUNNING
  (if (`self.LegendState`)
    (if (`self.IsRunning`)
      (`KismetSystemLibrary.Delay` 1.0)
      (if (<= (`self.CurrentStamina`) 0.0)
        (set `self.IsRunning` false)
        (set `CharacterMovementComponent.MaxWalkSpeed` 600.0 (`self.CharacterMovement`))
        (else
          (set `self.CurrentStamina` (- (`self.CurrentStamina`) 1.0))))
      (else
        (`|ExecutionSequence`
          (:`then_0`
            ;;[1 1 1] LEGEND STATE RECOVER
            (`KismetSystemLibrary.Delay` 1.0)
            (if (< (`self.CurrentStamina`) (`self.MaxStamina`))
              (bind _output_get (set `self.CurrentStamina` (+ (`self.CurrentStamina`) (* (`self.RecoverStamina`) 2.0))))
              (`KismetSystemLibrary.PrintString` (`KismetStringLibrary.Concat_StrStr` "STAMINA: " (`KismetStringLibrary.Conv_DoubleToString` _output_get)))
              (if (>= (`self.CurrentStamina`) 50.0)
                (set `self.CurrentStamina` 50.0))))
          (:`then_1`
            ;;[1 1 1] legend state walk faster
            (set `CharacterMovementComponent.MaxWalkSpeed` 1350.0 (`self.CharacterMovement`))))))
    (else
      (`|ExecutionSequence`
        (:`then_0`
          (if (`self.IsRunning`)
            (`KismetSystemLibrary.Delay` 1.0)
            (if (<= (`self.CurrentStamina`) 0.0)
              (set `self.IsRunning` false)
              (set `CharacterMovementComponent.MaxWalkSpeed` 600.0 (`self.CharacterMovement`))
              (else
                (set `self.CurrentStamina` (- (`self.CurrentStamina`) 1.0))))
            (else
              (`KismetSystemLibrary.Delay` 1.0)
              (if (< (`self.CurrentStamina`) (`self.MaxStamina`))
                (bind _output_get_2 (set `self.CurrentStamina` (+ (`self.CurrentStamina`) (`self.RecoverStamina`))))
                (`KismetSystemLibrary.PrintString` (`KismetStringLibrary.Concat_StrStr` "STAMINA: " (`KismetStringLibrary.Conv_DoubleToString` _output_get_2)))
                (if (>= (`self.CurrentStamina`) 50.0)
                  (set `self.CurrentStamina` 50.0))))))))))

(event `self.ReceiveAnyDamage`
  (params (Damage :type "Float (single-precision)") (DamageType :type "DamageType Object Reference") (InstigatedBy :type "Controller Object Reference") (DamageCauser :type "Actor Object Reference"))
  (bind _returnvalue (`GameplayStatics.GetPlayerController` 0))
  ;[1 1 1] RECEIVE DAMAGE
  (if (`self.isImmune`)
    _
    (elif (> (`self.Shield`) 0.0)
      (`KismetSystemLibrary.Delay` 0.1)
      (bind _output_get (set `self.Shield` (- (`self.Shield`) Damage)))
      (if (<= _output_get 0.0)
        (`KismetSystemLibrary.Delay` 0.1)
        (set `self.CurrentHealth` (+ (`self.CurrentHealth`) _output_get))
        (set `self.LegendStatePoints` (+ (`self.LegendStatePoints`) 10.0)))
      (elif (< (`self.CurrentHealth`) 30.0)
        (`KismetSystemLibrary.Delay` 0.1)
        (bind _output_get_2 (set `self.CurrentHealth` (- (`self.CurrentHealth`) (* Damage 0.95))))
        (set `self.LegendStatePoints` (+ (`self.LegendStatePoints`) 10.0))
        (if (<= _output_get_2 0.0)
          (set `self.Death` true)
          (`CharacterMovementComponent.DisableMovement` (`self.CharacterMovement`))
          (`KismetSystemLibrary.Delay` 2.0)
          (bind _returnvalue_2 (`|CreateWidget` "/Game/UserInterface/UI_DeadMenu.UI_DeadMenu_C"))
          (`UserWidget.AddToViewport` _returnvalue_2 0)
          (`WidgetBlueprintLibrary.SetInputMode_UIOnlyEx` _returnvalue null)
          (`GameplayStatics.SetGamePaused` true)
          (set `PlayerController.bShowMouseCursor` true _returnvalue)
          (else
            (`KismetSystemLibrary.PrintString` (`KismetStringLibrary.Conv_DoubleToString` _output_get_2))))
        (else
          (`KismetSystemLibrary.Delay` 0.1)
          (bind _output_get_3 (set `self.CurrentHealth` (- (`self.CurrentHealth`) Damage)))
          (set `self.LegendStatePoints` (+ (`self.LegendStatePoints`) 10.0))
          (if (<= _output_get_3 0.0)
            (`KismetSystemLibrary.PrintString` "U DEAD")
            (set `self.Death` true)
            (`CharacterMovementComponent.DisableMovement` (`self.CharacterMovement`))
            (`KismetSystemLibrary.Delay` 2.0)
            (bind _returnvalue_3 (`|CreateWidget` "/Game/UserInterface/UI_DeadMenu.UI_DeadMenu_C"))
            (`UserWidget.AddToViewport` _returnvalue_3 0)
            (`GameplayStatics.SetGamePaused` true)
            (set `PlayerController.bShowMouseCursor` true (`GameplayStatics.GetPlayerController` 0))
            (else
              (`KismetSystemLibrary.PrintString` (`KismetStringLibrary.Conv_DoubleToString` _output_get_3)))))))))

(fn `UserConstructionScript`)