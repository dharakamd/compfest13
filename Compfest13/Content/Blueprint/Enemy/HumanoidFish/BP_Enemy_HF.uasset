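; BP_Enemy_HF is the humanoid fish enemy Blueprint, handling the damage it receives and its death.
; On any damage, it waits briefly, subtracts the damage from Health, then adds LegendStatePoints to the player's BP_Character.
; It destroys itself once Health reaches zero or below, a check that only runs if the player character cast succeeds.
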(event `self.ReceiveAnyDamage`
  (params (Damage :type "Float (single-precision)") (DamageType :type "DamageType Object Reference") (InstigatedBy :type "Controller Object Reference") (DamageCauser :type "Actor Object Reference"))
  ;[1 1 1] ENEMY RECEIVE DAMAGE
  (`KismetSystemLibrary.Delay` 0.3)
  (set `self.Health` (- (`self.Health`) Damage))
  (bind _asbp_character (cast `/Game/Blueprint/MainCharacter/BP_Character` (`GameplayStatics.GetPlayerCharacter` 0)))
  (set `/Game/Blueprint/MainCharacter/BP_Character.LegendStatePoints` (+ (`/Game/Blueprint/MainCharacter/BP_Character.LegendStatePoints` _asbp_character) 5.0) _asbp_character)
  (if (<= (`self.Health`) 0.0)
    (`self.K2_DestroyActor`)))

(fn `UserConstructionScript`)