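; Player character with movement, look, stamina and health, plus a timed Legend State powered by points from attacking and taking damage.
; Attack, dash and running spend stamina, which Tick regenerates through one-second Delays, faster in Legend State, which also boosts run speed.
; Full-stamina-cost dashes grant damage immunity, cleared only on the forward branch.
; Debug keys alter stats; attack and death are only stat changes or prints.
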(event `Key|H`
  (params (Key :type "Key Structure"))
  ;[1 1 1] CHEAT
  (:`Pressed`
    (set `self.CurrentHealth` (- (`self.CurrentHealth`) 10.0))))

(event `Key|G`
  (params (Key :type "Key Structure"))
  ;[1 1 1] CHEAT
  (:`Pressed`
    (set `self.CurrentStamina` (- (`self.CurrentStamina`) 20.0))
    (if (<= (`self.CurrentStamina`) 0.0)
      (set `self.CurrentStamina` 0.0))))

(event `InputAxis|Move_ForwardBackward`
  (params (AxisValue :type "Float (single-precision)"))
  ;[0.8021 0.8013 0.7534] BASIC MOVEMENT
  (bind _output_get (set `self.ForwardIndex` AxisValue))
  (`self.AddMovementInput` (`self.GetActorForwardVector`) _output_get))

(event `Key|L`
  (params (Key :type "Key Structure"))
  ;[1 1 1] CHEAT
  (:`Pressed`
    (set `self.LegendStatePoints` (+ (`self.LegendStatePoints`) 50.0))
    (if (>= (`self.LegendStatePoints`) 100.0)
      (set `self.LegendStatePoints` 100.0))))

(event `InputAxis|Rotate_UpDown`
  (params (AxisValue :type "Float (single-precision)"))
  ;[0.8021 0.8013 0.7534] BASIC MOVEMENT
  (`self.AddControllerPitchInput` AxisValue))

(event `InputAxis|Move_RightLeft`
  (params (AxisValue :type "Float (single-precision)"))
  ;[0.8021 0.8013 0.7534] BASIC MOVEMENT
  (bind _output_get (set `self.RightIndex` AxisValue))
  (`self.AddMovementInput` (`self.GetActorRightVector`) _output_get))

(event `InputAxis|Rotate_RightLeft`
  (params (AxisValue :type "Float (single-precision)"))
  ;[0.8021 0.8013 0.7534] BASIC MOVEMENT
  (`self.AddControllerYawInput` AxisValue))

(event `InputAction|Attack`
  (params (Key :type "Key Structure"))
  ;[1 1 1] ATTACK
  (:`Pressed`
    (if (>= (`self.CurrentStamina`) 10.0)
      (set `self.CurrentStamina` (- (`self.CurrentStamina`) 10.0))
      (if (>= (`self.LegendStatePoints`) 100.0)
        (bind _output_get (set `self.LegendStatePoints` 100.0))
        (`KismetSystemLibrary.PrintString` (`KismetStringLibrary.Conv_DoubleToString` _output_get))
        (else
          (bind _output_get_2 (set `self.LegendStatePoints` (+ (`self.LegendStatePoints`) 5.0)))
          (`KismetSystemLibrary.PrintString` (`KismetStringLibrary.Conv_DoubleToString` _output_get_2)))))))

(event `Key|LeftAlt`
  (params (Key :type "Key Structure"))
  (:`Pressed`
    (set `self.bUseControllerRotationYaw` false))
  (:`Released`
    (set `self.bUseControllerRotationYaw` true)))

(event `InputAction|Dash`
  (params (Key :type "Key Structure"))
  ;[0.4463 0.9602 1] DASH
  (:`Pressed`
    (if (>= (`self.CurrentStamina`) 5.0)
      (set `self.CurrentStamina` (- (`self.CurrentStamina`) 5.0))
      (set `self.isImmune` true)
      (`KismetSystemLibrary.PrintString` "IS IMMUNE")
      (`|ExecutionSequence`
        (:`then_0`
          (if (>= (`self.ForwardIndex`) 1.0)
            (`self.LaunchCharacter` (* (`SceneComponent.GetForwardVector` (`self.CapsuleComponent`)) 5000.0))
            (`KismetSystemLibrary.Delay` 2.0)
            (set `self.isImmune` false)
            (`KismetSystemLibrary.PrintString` "IS NOT IMMUNE")))
        (:`then_1`
          (if (<= (`self.ForwardIndex`) -1.0)
            (`self.LaunchCharacter` (* (`SceneComponent.GetForwardVector` (`self.CapsuleComponent`)) -5000.0))))
        (:`then_2`
          (if (>= (`self.RightIndex`) 1.0)
            (`self.LaunchCharacter` (* (`SceneComponent.GetRightVector` (`self.CapsuleComponent`)) 5000.0))))
        (:`then_3`
          (if (<= (`self.RightIndex`) -1.0)
            (`self.LaunchCharacter` (* (`SceneComponent.GetRightVector` (`self.CapsuleComponent`)) -5000.0)))))
      (elif (and (< (`self.CurrentStamina`) 5.0) (> (`self.CurrentStamina`) 0.0))
        (set `self.CurrentStamina` (- (`self.CurrentStamina`) (`self.CurrentStamina`)))
        (`|ExecutionSequence`
          (:`then_0`
            (if (>= (`self.ForwardIndex`) 1.0)
              (`self.LaunchCharacter` (* (`SceneComponent.GetForwardVector` (`self.CapsuleComponent`)) 3750.0))))
          (:`then_1`
            (if (<= (`self.ForwardIndex`) -1.0)
              (`self.LaunchCharacter` (* (`SceneComponent.GetForwardVector` (`self.CapsuleComponent`)) -3750.0))))
          (:`then_2`
            (if (>= (`self.RightIndex`) 1.0)
              (`self.LaunchCharacter` (* (`SceneComponent.GetRightVector` (`self.CapsuleComponent`)) 3750.0))))
          (:`then_3`
            (if (<= (`self.RightIndex`) -1.0)
              (`self.LaunchCharacter` (* (`SceneComponent.GetRightVector` (`self.CapsuleComponent`)) -3750.0)))))))))

(event `InputAction|Run`
  (params (Key :type "Key Structure"))
  (bind _charactermovement (`self.CharacterMovement`))
  ;[1 1 1] RUN
  (:`Pressed`
    (if (and (> (`self.CurrentStamina`) 0.0) (> (`self.ForwardIndex`) 0.0))
      (set `self.IsRunning` true)
      (if (`self.LegendState`)
        ;;[1 1 1] LEGEND STATE RUN
        (set `CharacterMovementComponent.MaxWalkSpeed` 10000.0 _charactermovement)
        (else
          (set `CharacterMovementComponent.MaxWalkSpeed` 2000.0 _charactermovement))))))

(event `Key|W`
  (params (Key :type "Key Structure"))
  ;[1 1 1] RUN
  (:`Released`
    (set `self.IsRunning` false :!label _label)
    (set `CharacterMovementComponent.MaxWalkSpeed` 600.0 (`self.CharacterMovement`))))

(event `self.ReceiveAnyDamage`
  (params (Damage :type "Float (single-precision)") (DamageType :type "DamageType Object Reference") (InstigatedBy :type "Controller Object Reference") (DamageCauser :type "Actor Object Reference"))
  ;[1 1 1] RECEIVE DAMAGE
  (if (`self.isImmune`)
    _
    (elif (< (`self.CurrentHealth`) 30.0)
      (bind _output_get (set `self.CurrentHealth` (- (`self.CurrentHealth`) (* Damage 0.95))))
      (set `self.LegendStatePoints` (+ (`self.LegendStatePoints`) 10.0))
      (if (<= _output_get 0.0)
        (`KismetSystemLibrary.PrintString` "U DEAD"))
      (else
        (bind _output_get_2 (set `self.CurrentHealth` (- (`self.CurrentHealth`) Damage)))
        (set `self.LegendStatePoints` (+ (`self.LegendStatePoints`) 10.0))
        (if (<= _output_get_2 0.0)
          (`KismetSystemLibrary.PrintString` "U DEAD"))))))

(event `Key|S`
  (params (Key :type "Key Structure"))
  ;[1 1 1] RUN
  (:`Pressed`
    (goto _label)))

(event `InputAction|Legend State`
  (params (Key :type "Key Structure"))
  ;[0.8333 0.3559 0.3869] LEGEND STATE
  (:`Pressed`
    (if (>= (`self.LegendStatePoints`) 100.0)
      (set `self.LegendState` true)
      (`KismetSystemLibrary.PrintString` "LEGEND STATE")
      (`|ExecutionSequence`
        (:`then_0`
          (set `self.LegendStatePoints` 0.0)
          (`KismetSystemLibrary.Delay` 5.0)
          (set `self.LegendState` false)
          (`KismetSystemLibrary.PrintString` "LEGEND STATE IS OVER"))
        (:`then_1`
          (set `self.CurrentStamina` (+ (`self.CurrentStamina`) (* (`self.RecoverStamina`) 2.0))))))))

(event `self.ReceiveTick`
  (params (DeltaSeconds :type "Float (single-precision)"))
  ;[1 0.9498 0.3181] RECOVER STAMINA & DECREASE WHEN RUNNING
  (if (`self.LegendState`)
    (if (`self.IsRunning`)
      (`KismetSystemLibrary.Delay` 1.0)
      (if (<= (`self.CurrentStamina`) 0.0)
        (set `self.IsRunning` false)
        (set `CharacterMovementComponent.MaxWalkSpeed` 600.0 (`self.CharacterMovement`))
        (else
          (set `self.CurrentStamina` (- (`self.CurrentStamina`) 1.0))))
      (else
        ;;[1 1 1] LEGEND STATE RECOVER
        (`KismetSystemLibrary.Delay` 1.0)
        (if (< (`self.CurrentStamina`) (`self.MaxStamina`))
          (bind _output_get (set `self.CurrentStamina` (+ (`self.CurrentStamina`) (* (`self.RecoverStamina`) 2.0))))
          (`KismetSystemLibrary.PrintString` (`KismetStringLibrary.Concat_StrStr` "STAMINA: " (`KismetStringLibrary.Conv_DoubleToString` _output_get)))
          (if (>= (`self.CurrentStamina`) 50.0)
            (set `self.CurrentStamina` 50.0)))))
    (else
      (`|ExecutionSequence`
        (:`then_0`
          (if (`self.IsRunning`)
            (`KismetSystemLibrary.Delay` 1.0)
            (if (<= (`self.CurrentStamina`) 0.0)
              (set `self.IsRunning` false)
              (set `CharacterMovementComponent.MaxWalkSpeed` 600.0 (`self.CharacterMovement`))
              (else
                (set `self.CurrentStamina` (- (`self.CurrentStamina`) 1.0))))
            (else
              (`KismetSystemLibrary.Delay` 1.0)
              (if (< (`self.CurrentStamina`) (`self.MaxStamina`))
                (bind _output_get_2 (set `self.CurrentStamina` (+ (`self.CurrentStamina`) (`self.RecoverStamina`))))
                (`KismetSystemLibrary.PrintString` (`KismetStringLibrary.Concat_StrStr` "STAMINA: " (`KismetStringLibrary.Conv_DoubleToString` _output_get_2)))
                (if (>= (`self.CurrentStamina`) 50.0)
                  (set `self.CurrentStamina` 50.0))))))))))

(fn `UserConstructionScript`)